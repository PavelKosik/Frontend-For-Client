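; BP_SaveInteract is an interactable save point that saves the player's game when used.
; On interact, it gets the save object from the GameInstance, writes the SavePosition transform, save name and level name, then saves it.
; A looping Delay and FlipFlop flickers the PointLight as feedback, with the loop counter also blocking retriggers.
; Without a valid save object, it prints an error about joining from the main menu.
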(event EventBeginPlay
  (|CallParentFunction) ; This node is disabled and will not be called.\nDrag off pins to build functionality.
)

(event EventOnInteract
  (bind _pointlight (Variables|Default|GetPointLight))
  ;[1 1 1] Override OnInteract and called from Controller
  (if (<= (Variables|Default|GetNumSaveEffect) 0)
    (bind _mygamesave (Class|BPMainMenuInterface|MSGGetGameInstanceVariables(Message) (Game|GetGameInstance)))
    (Utilities|IsValid _mygamesave
      (:Is%20Valid
        (Variables|/Game/AntizeMenuSystemSolo/Blueprints/SaveGame/BP_MySaveGame.BP_MySaveGame_C|SetPlayerPosition _mygamesave (Transformation|GetWorldTransform (Variables|Default|GetSavePosition)))
        (Variables|/Game/AntizeMenuSystemSolo/Blueprints/SaveGame/BP_MySaveGame.BP_MySaveGame_C|SetGameName _mygamesave (Variables|Default|GetSaveName))
        (Variables|/Game/AntizeMenuSystemSolo/Blueprints/SaveGame/BP_MySaveGame.BP_MySaveGame_C|SetLevelName _mygamesave (Variables|Default|GetLevelName))
        (CallFunction|SaveGame _mygamesave)
        ;[1 1 1] Make an effect on save
        (Variables|Default|SetNumSaveEffect 0)
        (Utilities|FlowControl|Delay 0.05 :!label _label)
        (Utilities|FlowControl|FlipFlop
          (:A
            (Rendering|SetVisibility _pointlight true false))
          (:B
            (Rendering|SetVisibility _pointlight false false)))
        (if (<= (Variables|Default|GetNumSaveEffect) 10)
          (Math|Integer|IncrementInt (Variables|Default|GetNumSaveEffect)
            (:%20%20
              (goto _label)))
          (else
            (Rendering|SetVisibility (Variables|Default|GetPointLight) false false)
            (Variables|Default|SetNumSaveEffect 0))))
      (:Is%20Not%20Valid
        (Development|PrintString "Error on save, need to join from Main menu")))))

(fn ConstructionScript
  (|CallParentFunction))